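; Receiver_BP is a networked actor that mirrors a transform received over UDP.
; Incoming bytes are converted to a JSON string and parsed into an ID and transform struct.
; Each tick, if the received ID matches the actor's own ID, it sets the root component's world transform, without sweep or interpolation.
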(event `self.ReceiveTick`
  (params (DeltaSeconds :type "Float (single-precision)"))
  (bind (_id _transform) (break `/Game/Dev/Blueprints/Networking/IDTransf_str` (`self.IDTransf`)))
  ;[1 1 1] Sets the transform for the sceneComponent if the ID's match
  (if (== (`self.ID`) _id)
    (`SceneComponent.K2_SetWorldTransform` (`self.DefaultSceneRoot`) _transform false false)))

(event `self.UDP.OnReceivedBytes`
  (params (Bytes :type "Array of Byte (by ref)"))
  ;[1 1 1] Transforms the received bytes to the struct
  (`SIOJLibrary.JsonObjectToStruct` (`SIOJLibrary.Conv_JsonValueToJsonObject` (`SIOJsonValue.ValueFromJsonString` (`CoreUtilityBPLibrary.Conv_BytesToString` Bytes))) (`self.IDTransf`)))

(fn `UserConstructionScript`)