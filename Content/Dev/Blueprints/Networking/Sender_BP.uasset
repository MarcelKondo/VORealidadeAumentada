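; Sender_BP is a networking actor that broadcasts its ID and world transform over UDP.
; On BeginPlay a looping timer fires SendData at the configured interval.
; Each send packs the ID and root component transform into a struct, encodes it as JSON, converts it to bytes and emits it through the UDP component.
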(event `self.ReceiveBeginPlay`
  ;[1 1 1] Sets the interval in which to send the data
  (`KismetSystemLibrary.K2_SetTimerDelegate` (delegate `SendData`) (`self.SendInterval`) true))

(event `SendData`
  ;[1 1 1] Encodes the strucure and emits it
  (bind _output_get (set `self.IDTransf` (make `/Game/Dev/Blueprints/Networking/IDTransf_str` (`self.ID`) (`SceneComponent.K2_GetComponentToWorld` (`self.DefaultSceneRoot`)))))
  (`UDPComponent.Emit` (`self.UDP`) (`CoreUtilityBPLibrary.Conv_StringToBytes` (`SIOJsonObject.EncodeJson` (`SIOJLibrary.StructToJsonObject` _output_get)))))

(fn `UserConstructionScript`)