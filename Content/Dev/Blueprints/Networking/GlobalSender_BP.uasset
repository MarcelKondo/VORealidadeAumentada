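; GlobalSender_BP is a networking actor that gathers all Sender_BP actors in its construction script to serialize their state.
; A looping timer started on BeginPlay calls SendData every SendInterval, which uses EncodeArray to append each sender's ID and transform into one string.
; The UDP emit of that string is disconnected, so nothing is transmitted.
; SortByID is an unfinished, uncalled stub.
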(event `self.ReceiveBeginPlay`
  (`KismetSystemLibrary.K2_SetTimerDelegate` (delegate `SendData`) (`self.SendInterval`) true))

(event `SendData`
  (bind _sring (`self.EncodeArray` (`self.TrackedActors`))))

(fn `EncodeArray`
  (params (Actors :type "Array of Actor Object Reference"))
  (returns (Sring :type String))
  (locals (ResultingString :type String))
  (for _array_element Actors
    (bind _assender_bp (cast `/Game/Dev/Blueprints/Networking/Sender_BP` _array_element)
      (:`then`
        (bind _output_get (set `local.ResultingString` (`KismetStringLibrary.Concat_StrStr` (`local.ResultingString`) "ID: " (`KismetStringLibrary.Conv_ByteToString` (`/Game/Dev/Blueprints/Networking/Sender_BP.ID` _assender_bp)) (`KismetStringLibrary.Conv_TransformToString` (`self.GetTransform` _assender_bp))))))
      (:`CastFailed`
        (`KismetSystemLibrary.PrintString` "GlobalSender_BP -> EncodeArray: found actor that is not a Sender_BP" false true (struct :`R` 1.0 :`G` 0.963404 :`A` 1.0)))))
  (return _output_get))

(fn `SortByID`
  (for _array_element (`self.TrackedActors`)
    (cast `/Game/Dev/Blueprints/Networking/Sender_BP` _array_element)))

(fn `UserConstructionScript`
  (bind _outactors (`GameplayStatics.GetAllActorsOfClass` "/Game/Dev/Blueprints/Networking/Sender_BP.Sender_BP_C"))
  (set `self.TrackedActors` _outactors))