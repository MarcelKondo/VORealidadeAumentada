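; Planet actor for the AugmentedUnrealityExample project, configured by orbit distance, radius and rotation rate.
; The construction script offsets the mesh along X by the orbit distance, lowers it by the radius and scales it to that radius.
; It also feeds the rotation rate to a RotatingMovement component as yaw spin.
; BeginPlay gives the mesh a random yaw, varying its facing without moving it along the orbit.
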(event `self.ReceiveBeginPlay`
  (`SceneComponent.K2_SetRelativeRotation` (`self.PlanetMesh`) (`KismetMathLibrary.MakeRotator` 0.0 0.0 (`KismetMathLibrary.RandomFloatInRange` -180.0 180.0)) false false))

(fn `UserConstructionScript`
  (bind _radius (`self.Radius`))
  (bind _planetmesh (`self.PlanetMesh`))
  (`SceneComponent.K2_SetRelativeLocation` _planetmesh (`KismetMathLibrary.MakeVector` (`self.Orbit`) 0.0 (* _radius -1.0)) false false)
  (`SceneComponent.SetRelativeScale3D` _planetmesh (`KismetMathLibrary.Conv_DoubleToVector` (/ _radius 25.0)))
  (set `RotatingMovementComponent.RotationRate` (`KismetMathLibrary.MakeRotator` 0.0 0.0 (`self.RotationRate`)) (`self.RotatingMovement`)))